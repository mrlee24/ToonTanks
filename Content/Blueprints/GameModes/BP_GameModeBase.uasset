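; BP_GameModeBase is a game mode Blueprint that puts the start, end and score UI on screen.
; GameStart creates WBP_GameStart with the StartDelay value, and GameOver creates WBP_GameStop with the PlayerWon result.
; Tick creates and adds a new WBP_Score widget each time it fires, with no guard against duplicates.
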(event EventGameStart
  (bind _returnvalue (UserInterface|CreateWidget "/Game/Blueprints/Widgets/WBP_GameStart.WBP_GameStart_C"))
  (Default|SetStartDelay _returnvalue (Variables|Default|GetStartDelay))
  (UserInterface|Viewport|AddtoViewport _returnvalue 0))

(event EventGameOver
  (params (PlayerWon :type Boolean))
  (bind _returnvalue (UserInterface|CreateWidget "/Game/Blueprints/Widgets/WBP_GameStop.WBP_GameStop_C"))
  (Default|SetPlayerWon _returnvalue PlayerWon)
  (UserInterface|Viewport|AddtoViewport _returnvalue 0))

(event EventTick
  (params (DeltaSeconds :type Float%20%28single-precision%29))
  (bind _returnvalue (UserInterface|CreateWidget "/Game/Blueprints/Widgets/WBP_Score.WBP_Score_C"))
  (UserInterface|Viewport|AddtoViewport _returnvalue 0))

(fn ConstructionScript)